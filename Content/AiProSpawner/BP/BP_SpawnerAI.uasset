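; BP_SpawnerAI spawns random AI classes at random reachable navmesh points around spawn point actors, in waves, as a respawning population, or on trigger.
; BeginPlay or StartWaves begins delayed spawning; TriggerSpawn uses the trigger's own spawn points and supplied classes.
; A delayed CheckHowManyAiIsAlive loop polls living AI through GetAllActorsOfClass, respawning losses or starting the next wave once all are dead.
; Waves grow up to a cap, and waves and respawns can be limited or infinite.
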(event Custom|First%20Wave
  ;[0 0 0] Waves system and respawn
  ;;[0 0 0] Start a wave
  (Variables|Default|SetWavesStarting? true)
  (bind _spawn_ai (CallFunction|SpawnWave (Variables|Default|GetNumber%20Of%20AI%20To%20Spawn)))
  (if _spawn_ai
    (Variables|Default|SetWaves (+ (Variables|Default|GetWaves) 1))
    (if (>= (Variables|Default|GetNumber%20ai%20to%20spawn%20Left) 1) :!label _label
      (Utilities|FlowControl|Delay (Variables|Default|GetDelay%20between%20each%20ai%20spawn))
      (bind _spawn_ai__ (CallFunction|SpawnAiWave))
      (if _spawn_ai__
        (goto _label)
        (else
          (CallFunction|CheckHowManyAiIsAlive))))))

(event Custom|Respawn
  ;[0 0 0] Waves system and respawn
  ;;[0 0 0] Respawn ai
  (if (Variables|Default|GetRespawn%20infinite?)
    (Utilities|FlowControl|Delay (Variables|Default|GetDelay%20For%20Respawn) :!label _label)
    (CallFunction|SpawnAI 1)
    (elif (<= (Variables|Default|GetLimit%20of%20Ai%20respawn) 0)
      (Utilities|FlowControl|Delay 0.1)
      (CallFunction|CheckHowManyAiIsAlive)
      (else
        (Math|Integer|DecrementInt (Variables|Default|GetLimit%20of%20Ai%20respawn)
          (:%20%20
            (goto _label)))))))

(event Custom|Check%20how%20many%20ai%20is%20alive
  ;[0 0 0] Waves system and respawn
  ;;[0 0 0] Check ai alive and start wave or respawn ai
  (bind _all_dead_ (CallFunction|CheckAiAlive))
  (if (Variables|Default|GetWaves%20System)
    (if (Variables|Default|GetWavesStarting?)
      (if _all_dead_
        (if (Variables|Default|GetStop%20Waves)
          (Utilities|FlowControl|Delay 0.1 :!label _label)
          (CallFunction|CheckHowManyAiIsAlive)
          (else
            (CallFunction|StartAWave)))
        (else
          (goto _label))))
    (elif (< (Variables|Default|GetAll%20AI%20Alive) (Variables|Default|GetNumber%20Of%20AI%20To%20Spawn))
      (if (Variables|Default|GetAi%20Respawn?)
        (CallFunction|Respawn)
        (else
          (Utilities|FlowControl|Delay 0.1 :!label _label_2)
          (CallFunction|CheckHowManyAiIsAlive)))
      (else
        (goto _label_2)))))

(event Custom|StartingServer
  ;[0 0 0] Event begin play and start
  ;;[0 0 0] Start spawner
  (Utilities|FlowControl|DoOnce false
    (:Completed
      (if (not (Variables|Default|GetStartWavesWithTrigger))
        (if (Variables|Default|GetWaves%20System)
          (Utilities|FlowControl|Delay (Variables|Default|GetDelay%20Before%20Spawn))
          (CallFunction|FirstWave)
          (elif (not (Variables|Default|GetSpawnAI%20On%20Trigger?))
            (Utilities|FlowControl|Delay (Variables|Default|GetDelay%20Before%20Spawn))
            (CallFunction|SpawnAI (Variables|Default|GetNumber%20Of%20AI%20To%20Spawn))))))))

(event Custom|Start%20a%20wave
  ;[0 0 0] Waves system and respawn
  ;;[0 0 0] Start a wave
  (if (not (Variables|Default|GetStop%20Waves))
    (bind _start_a_wave__ (CallFunction|CheckifStartAWave))
    (if _start_a_wave__
      (Utilities|FlowControl|Delay (Variables|Default|GetDelay%20for%20the%20next%20waves))
      (bind _number_ai_to_spawn (CallFunction|HowManySpawnAiWave))
      (bind _spawn_ai (CallFunction|SpawnWave _number_ai_to_spawn))
      (if _spawn_ai
        (Variables|Default|SetWaves (+ (Variables|Default|GetWaves) 1))
        (if (>= (Variables|Default|GetNumber%20ai%20to%20spawn%20Left) 1) :!label _label
          (Utilities|FlowControl|Delay (Variables|Default|GetDelay%20between%20each%20ai%20spawn))
          (bind _spawn_ai__ (CallFunction|SpawnAiWave))
          (if _spawn_ai__
            (goto _label)
            (else
              (CallFunction|CheckHowManyAiIsAlive)))))
      (else
        (Variables|Default|SetStop%20Waves true)
        (Utilities|FlowControl|Delay 0.5)
        (CallFunction|CheckHowManyAiIsAlive)))))

(event Custom|Trigger%20Spawn
  (params (Number%20to%20spawn :type Integer) (Trigger :type BP%20Trigger%20Spawn%20Object%20Reference) (Ai%20to%20spawn :type Array%20of%20Actor%20Class%20References) (Delay%20before%20spawn%20ai :type Float%20%28single-precision%29))
  ;[0 0 0] On Trigger Spawn AI
  (if (Variables|Default|GetSpawnAI%20On%20Trigger?)
    (Variables|Default|SetTrigger Trigger)
    (Utilities|FlowControl|Delay Delay%20before%20spawn%20ai)
    (CallFunction|SpawnAITrigger Number%20to%20spawn Ai%20to%20spawn)))

(event Custom|StartWaves
  ;[0 0 0] Event begin play and start
  ;;[0 0 0] Start spawner
  (if (Variables|Default|GetWaves%20System)
    (Utilities|FlowControl|Delay (Variables|Default|GetDelay%20Before%20Spawn))
    (CallFunction|FirstWave)))

(event EventBeginPlay
  ;[0 0 0] Event begin play and start
  ;;[0 0 0] Event begin play
  (CallFunction|StartingServer))

(fn ConstructionScript)

(fn SpawnWave
  (params (Number%20of%20ai :type Integer))
  (Variables|Default|SetNumber%20ai%20to%20spawn%20Left Number%20of%20ai)
  (if (Variables|Default|GetInifnite%20Waves?)
    (return true)
    (elif (>= (Variables|Default|GetWaves) (Variables|Default|GetNumber%20of%20waves))
      (Variables|Default|SetStop%20Waves true)
      (return false)
      (else
        (return true)))))

(fn CheckAiAlive
  (Variables|Default|SetAll%20AI%20Alive 0)
  (Variables|Default|Setone%20is%20alive%20? false)
  (bind _outactors (Actor|GetAllActorsOfClass "/Game/AiProSpawner/BP/Ai.Ai_C"))
  (for _array_element _outactors
    ;[1 0.2135 0.2135] Cast you AI Parent
    (if (not (Variables|/Game/AiProSpawner/BP/Ai.Ai_C|GetDead? _array_element))
      (Variables|Default|SetAll%20AI%20Alive (+ (Variables|Default|GetAll%20AI%20Alive) 1))
      (Variables|Default|Setone%20is%20alive%20? true)))
  (if (Variables|Default|Getone%20is%20alive%20?)
    (Variables|Default|SetAll%20dead? false)
    (return false)
    (elif (<= (Variables|Default|GetNumber%20ai%20to%20spawn%20Left) 0)
      (Variables|Default|SetAll%20dead? true)
      (return true)
      (else
        (Variables|Default|SetAll%20dead? false)
        (return false)))))

(fn CheckifStartAWave
  (if (Variables|Default|GetInifnite%20Waves?)
    (return true)
    (elif (>= (Variables|Default|GetWaves) (Variables|Default|GetNumber%20of%20waves))
      (return false)
      (else
        (return true)))))

(fn HowManySpawnAiWave
  (if (> (+ (Variables|Default|GetNumber%20Of%20AI%20To%20Spawn) (Variables|Default|GetNumber%20of%20ai%20add%20to%20next%20waves)) (Variables|Default|GetLimit%20Of%20The%20Max%20AI))
    (return (Variables|Default|GetLimit%20Of%20The%20Max%20AI))
    (else
      (bind _output_get (Variables|Default|SetNumber%20Of%20AI%20To%20Spawn (+ (Variables|Default|GetNumber%20Of%20AI%20To%20Spawn) (Variables|Default|GetNumber%20of%20ai%20add%20to%20next%20waves))))
      (return _output_get))))

(fn SpawnAI
  (params (Number%20of%20ai :type Integer))
  (bind _class_of_actor_to_spawn (Variables|Default|GetClass%20Of%20Actor%20To%20Spawn))
  (bind _spawn_points (Variables|Default|GetSpawn%20Points))
  (bind _returnvalue (Utilities|Array|LastIndex _spawn_points))
  (bind _returnvalue_2 (Math|Random|RandomIntegerinRange 0 _returnvalue))
  (bind _output (Utilities|Array|Get(acopy) _spawn_points _returnvalue_2))
  (bind _returnvalue_3 (Transformation|GetActorLocation _output))
  (bind _radius_of_spawner (Variables|/Game/AiProSpawner/BP/BP_SpawnPoint.BP_SpawnPoint_C|GetRadius%20Of%20Spawner _output))
  (bind _randomlocation (AI|Navigation|GetRandomReachablePointinRadius (Math|Vector|MakeVector (.x _returnvalue_3) (.y _returnvalue_3) (.z _returnvalue_3)) _radius_of_spawner 0 0))
  (Variables|Default|SetNumber%20ai%20to%20spawn%20Left Number%20of%20ai)
  (for _index (range 1 Number%20of%20ai)
    (bind _returnvalue_4 (Game|SpawnActorfromClass (Utilities|Array|Get(acopy) _class_of_actor_to_spawn (Math|Random|RandomIntegerinRange 0 (Utilities|Array|LastIndex _class_of_actor_to_spawn))) (Math|Transform|MakeTransform (Math|Vector|MakeVector (.x _randomlocation) (.y _randomlocation) (+ (.z _randomlocation) 5e+01)) "0, 0, 0" "1,1,1") "AdjustIfPossibleButAlwaysSpawn" 0 0))
    (Utilities|Array|Add (Variables|Default|GetAll%20Ai%20Spawn) _returnvalue_4)
    (Variables|Default|SetNumber%20ai%20to%20spawn%20Left (- (Variables|Default|GetNumber%20ai%20to%20spawn%20Left) 1)))
  (CallFunction|CheckHowManyAiIsAlive))

(fn SpawnAiWave
  (bind _class_of_actor_to_spawn (Variables|Default|GetClass%20Of%20Actor%20To%20Spawn))
  (bind _spawn_points (Variables|Default|GetSpawn%20Points))
  (bind _returnvalue (Utilities|Array|LastIndex _spawn_points))
  (bind _returnvalue_2 (Math|Random|RandomIntegerinRange 0 _returnvalue))
  (bind _output (Utilities|Array|Get(acopy) _spawn_points _returnvalue_2))
  (bind _returnvalue_3 (Transformation|GetActorLocation _output))
  (bind _radius_of_spawner (Variables|/Game/AiProSpawner/BP/BP_SpawnPoint.BP_SpawnPoint_C|GetRadius%20Of%20Spawner _output))
  (bind _randomlocation (AI|Navigation|GetRandomReachablePointinRadius (Math|Vector|MakeVector (.x _returnvalue_3) (.y _returnvalue_3) (.z _returnvalue_3)) _radius_of_spawner 0 0))
  (bind _returnvalue_4 (Game|SpawnActorfromClass (Utilities|Array|Get(acopy) _class_of_actor_to_spawn (Math|Random|RandomIntegerinRange 0 (Utilities|Array|LastIndex _class_of_actor_to_spawn))) (Math|Transform|MakeTransform (Math|Vector|MakeVector (.x _randomlocation) (.y _randomlocation) (+ (.z _randomlocation) 5e+01)) "0, 0, 0" "1,1,1") "AdjustIfPossibleButAlwaysSpawn" 0 0))
  (Utilities|Array|Add (Variables|Default|GetAll%20Ai%20Spawn) _returnvalue_4)
  (bind _output_get (Variables|Default|SetNumber%20ai%20to%20spawn%20Left (- (Variables|Default|GetNumber%20ai%20to%20spawn%20Left) 1)))
  (CallFunction|CheckHowManyAiIsAlive)
  (return (>= _output_get 1)))

(fn SpawnAITrigger
  (params (Number%20of%20ai :type Integer) (Ai%20To%20Spawn :type Array%20of%20Actor%20Class%20References))
  (bind _trigger (Variables|Default|GetTrigger))
  (bind _spawnpoints (Variables|/Game/AiProSpawner/BP/BP_Trigger_Spawn.BP_Trigger_Spawn_C|GetSpawnPoints _trigger))
  (bind _returnvalue (Utilities|Array|LastIndex _spawnpoints))
  (bind _returnvalue_2 (Math|Random|RandomIntegerinRange 0 _returnvalue))
  (bind _output (Utilities|Array|Get(acopy) _spawnpoints _returnvalue_2))
  (bind _returnvalue_3 (Transformation|GetActorLocation _output))
  (bind _radius_of_spawner (Variables|/Game/AiProSpawner/BP/BP_SpawnPoint.BP_SpawnPoint_C|GetRadius%20Of%20Spawner _output))
  (bind _randomlocation (AI|Navigation|GetRandomReachablePointinRadius (Math|Vector|MakeVector (.x _returnvalue_3) (.y _returnvalue_3) (.z _returnvalue_3)) _radius_of_spawner 0 0))
  (for _index (range 1 Number%20of%20ai)
    (Game|SpawnActorfromClass (Utilities|Array|Get(acopy) Ai%20To%20Spawn (Math|Random|RandomIntegerinRange 0 (Utilities|Array|LastIndex Ai%20To%20Spawn))) (Math|Transform|MakeTransform (Math|Vector|MakeVector (.x _randomlocation) (.y _randomlocation) (+ (.z _randomlocation) 5e+01)) "0, 0, 0" "1,1,1") "AdjustIfPossibleButAlwaysSpawn" 0 0))
  (CallFunction|CheckHowManyAiIsAlive))