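; BP_Trigger_Spawn is a placeable trigger volume for the AiProSpawner system, meant to spawn AI or start waves through BP_SpawnerAI.
; The construction script applies the trigger's configurable scale, relative location and in-game visibility.
; A DoOnce chain calls TriggerSpawn or StartWaves on the first spawner found, depending on its SpawnAIOnTrigger and the trigger's StartWaves flag.
; That chain is disconnected behind an unset player cast, so overlapping currently does nothing.
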(event OnComponentBeginOverlap(Trigger)
  (params (OverlappedComponent :type Primitive%20Component%20Object%20Reference) (OtherActor :type Actor%20Object%20Reference) (OtherComp :type Primitive%20Component%20Object%20Reference) (OtherBodyIndex :type Integer) (bFromSweep :type Boolean) (SweepResult :type Hit%20Result%20Structure%20%28by%20ref%29))
  ;[0 0 0] On trigger spawn ai
)

(fn ConstructionScript
  ;[0 0 0] set trigger scale
  (Transformation|SetWorldScale3D (Variables|Default|GetTrigger) (Variables|Default|GetTrigger%20Scale))
  ;[0 0 0] Set the location of the trigger
  (Transformation|SetRelativeLocation (Variables|Default|GetTrigger) (Variables|Default|GetLocation%20Of%20The%20Trigger) false false)
  ;[0 0 0] See the trigger in game ?
  (if (Variables|Default|GetSee%20the%20trigger%20in%20game?)
    (Development|SetHiddeninGame (Variables|Default|GetTrigger) false false)
    (else
      (Development|SetHiddeninGame (Variables|Default|GetTrigger) true false))))